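; BP_Player is the player Blueprint, handling movement and look input plus restart and load hotkeys.
; Move, strafe and look axes drive movement input along control-rotation vectors and controller pitch and yaw.
; BeginPlay caches BP_GameInstance; R restarts through BP_GameMode and then calls CallOnLoad on the instance, while P calls only CallOnLoad.
; A disconnected debug loop would print the saved SCoin keys.
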(event `InputAxis|Move`
  (params (AxisValue :type "Float (single-precision)"))
  (`self.AddMovementInput` (`KismetMathLibrary.GetForwardVector` (`self.GetControlRotation`)) AxisValue))

(event `InputAxis|Straf`
  (params (AxisValue :type "Float (single-precision)"))
  (`self.AddMovementInput` (`KismetMathLibrary.GetRightVector` (`self.GetControlRotation`)) AxisValue))

(event `InputAxis|Look-Y`
  (params (AxisValue :type "Float (single-precision)"))
  (`self.AddControllerPitchInput` AxisValue))

(event `InputAxis|Look-X`
  (params (AxisValue :type "Float (single-precision)"))
  (`self.AddControllerYawInput` AxisValue))

(event `self.ReceiveBeginPlay`
  (bind _asbp_game_instance (cast `/Game/MyGame/Blueprints/Core/BP_GameInstance` (`GameplayStatics.GetGameInstance`)))
  (set `self.GameInstance` _asbp_game_instance))

(event `Key|R`
  (params (Key :type "Key Structure"))
  (:`Pressed`
    (bind _asbp_game_mode (cast `/Game/MyGame/Blueprints/Core/BP_GameMode` (`GameplayStatics.GetGameMode`)))
    (`GameMode.RestartGame` _asbp_game_mode)
    (`/Game/MyGame/Blueprints/Core/BP_GameInstance.OnLoad` (`self.GameInstance`) :!label _label)))

(event `Key|P`
  (params (Key :type "Key Structure"))
  (:`Pressed`
    (goto _label)))

(fn `UserConstructionScript`)